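; Flying Super Sonic player character for the Giganto boss fight, with camera-relative movement, a velocity-burst boost and a basic combo montage.
; BeginPlay locks onto the first Giganto; Tick eases control yaw toward its camera point, updates its homing icon and draws debug vectors.
; A squared-distance check drives the camera: beyond the threshold it shifts sideways with the close arm length, within it recenters with the far one and hides the icon.
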(event `self.ReceiveBeginPlay`
  (bind _outactors (`GameplayStatics.GetAllActorsOfClass` "/Game/Characters/Bosses/BP_Giganto.BP_Giganto_C"))
  (set `self.LockOnTarget` (`|GetArrayItem` _outactors))
  (set `self.OriginalRelativeCameraLocation` (`SceneComponent.RelativeLocation` (`self.FollowCamera`)))
  (set `self.FarCameraRelativeLocation` (`KismetMathLibrary.MakeVector` (.x (`self.OriginalRelativeCameraLocation`)) 150.0 (.z (`self.OriginalRelativeCameraLocation`)))))

(event `self.ReceiveTick`
  (params (DeltaSeconds :type "Float (single-precision)"))
  (bind _returnvalue (`self.K2_GetActorLocation`))
  (bind _returnvalue_2 (`self.K2_GetActorLocation`))
  (bind _returnvalue_3 (`self.K2_GetActorLocation`))
  (`/Engine/EditorBlueprintResources/StandardMacros.IsValid` (`self.LockOnTarget`)
    (:`Is Valid`
      (`self.SetCameraLocationAndRotation` DeltaSeconds (`self.LockOnTarget`))
      (`/Game/Characters/Bosses/BP_Giganto.SetHomingIconLocation` (`self.LockOnTarget`) self)
      (`/Game/Characters/Bosses/BP_Giganto.SetHomingIconVisibility` (`self.LockOnTarget`) (not (`self.InLockOnRange`)))
      (`KismetSystemLibrary.DrawDebugLine` (`self.K2_GetActorLocation`) (`/Game/Characters/Bosses/BP_Giganto.GetClosestLockOnPoint` (`self.LockOnTarget`) self) (struct :`G` 0.155862 :`B` 1.0 :`A` 1.0) 0.0 2.0)
      (`KismetSystemLibrary.DrawDebugArrow` _returnvalue_2 (+ _returnvalue_2 (* (`KismetMathLibrary.Normal` (`MovementComponent.Velocity` (`self.CharacterMovement`))) 150.0)) 0.0 (struct :`R` 1.0 :`G` 0.06301 :`A` 1.0) 0.0 2.0)
      (`KismetSystemLibrary.DrawDebugArrow` _returnvalue_3 (+ _returnvalue_3 (* (`self.GetActorForwardVector`) 150.0)) 0.0 (struct :`R` 0.030713 :`G` 1.0 :`A` 1.0) 0.0 2.0)
      (`KismetSystemLibrary.DrawDebugArrow` _returnvalue (+ _returnvalue (* (`self.GetActorRightVector`) 150.0)) 0.0 (struct :`R` 0.973446 :`G` 0.030713 :`B` 1.0 :`A` 1.0) 0.0 2.0))))

(event `InputAxis|MoveForward`
  (params (AxisValue :type "Float (single-precision)"))
  (if (not (`self.MovementBlocked`))
    (`self.AddMovementInput` (`KismetMathLibrary.GetForwardVector` (`KismetMathLibrary.MakeRotator` 0.0 0.0 (.yaw (`self.GetControlRotation`)))) AxisValue)))

(event `InputAxis|MoveRight`
  (params (AxisValue :type "Float (single-precision)"))
  (if (not (`self.MovementBlocked`))
    (`self.AddMovementInput` (`KismetMathLibrary.GetRightVector` (`KismetMathLibrary.MakeRotator` 0.0 0.0 (.yaw (`self.GetControlRotation`)))) AxisValue)))

(event `InputAction|Boost`
  (params (Key :type "Key Structure"))
  (bind _charactermovement (`self.CharacterMovement`))
  ;[1 1 1] TODO: Move to native C++
  (:`Pressed`
    (if (not (`self.MovementBlocked`))
      (bind _output_get (set `CharacterMovementComponent.MaxFlySpeed` 9000.0 (`self.CharacterMovement`)))
      (set `MovementComponent.Velocity` (`KismetMathLibrary.ClampVectorSize` (+ (`MovementComponent.Velocity` _charactermovement) (* (`self.GetActorForwardVector`) _output_get)) 0.0 (`CharacterMovementComponent.MaxFlySpeed` (`self.CharacterMovement`))) _charactermovement)))
  (:`Released`
    (set `CharacterMovementComponent.MaxFlySpeed` 4000.0 (`self.CharacterMovement`))))

(event `InputAction|BasicCombo`
  (params (Key :type "Key Structure"))
  ;[1 1 1] TODO: Move to native C++
  (:`Pressed`
    (if (not (`self.InputBlocked`))
      (message `/Game/Blueprints/Attacks/BPI_PlayAttackMontage.PlayComboMontage` (`SkeletalMeshComponent.GetAnimInstance` (`self.Mesh`)) "NewEnumerator0"))))

(fn `SetCameraLocation`
  (params (Target :type "Actor Object Reference") (DeltaTime :type "Float (double-precision)"))
  (bind _returnvalue (> (`KismetMathLibrary.VSizeSquared` (- (`self.K2_GetActorLocation` Target) (`self.K2_GetActorLocation`))) (* (`self.CameraZoomThreshhold`) (`self.CameraZoomThreshhold`))))
  (set `self.InLockOnRange` (not _returnvalue))
  (if _returnvalue
    (`SceneComponent.K2_SetRelativeLocation` (`self.FollowCamera`) (`KismetMathLibrary.VInterpTo` (`SceneComponent.RelativeLocation` (`self.FollowCamera`)) (`self.FarCameraRelativeLocation`) (`local.DeltaTime`) 2.0) false false)
    (set `SpringArmComponent.TargetArmLength` (`KismetMathLibrary.FInterpTo` (`SpringArmComponent.TargetArmLength` (`self.CameraBoom`)) (`self.CloseTargetArmLength`) (`local.DeltaTime`) 2.0) (`self.CameraBoom`))
    (else
      (`SceneComponent.K2_SetRelativeLocation` (`self.FollowCamera`) (`KismetMathLibrary.VInterpTo` (`SceneComponent.RelativeLocation` (`self.FollowCamera`)) (`self.OriginalRelativeCameraLocation`) (`local.DeltaTime`) 2.0) false false)
      (set `SpringArmComponent.TargetArmLength` (`KismetMathLibrary.FInterpTo` (`SpringArmComponent.TargetArmLength` (`self.CameraBoom`)) (`self.FarTargetArmLength`) (`local.DeltaTime`) 2.0) (`self.CameraBoom`)))))

(fn `SetCameraLocationAndRotation`
  (params (DeltaTime :type "Float (single-precision)") (Target :type "/Game/Characters/Bosses/BP_Giganto Object Reference"))
  (bind (_returnvalue_roll _returnvalue_pitch) (`KismetMathLibrary.BreakRotator` (`self.GetControlRotation`)))
  (bind (_returnvalue_roll_2 _returnvalue_pitch_2 _returnvalue_yaw) (`KismetMathLibrary.BreakRotator` (`KismetMathLibrary.FindLookAtRotation` (`self.K2_GetActorLocation`) (`SceneComponent.K2_GetComponentLocation` (`/Game/Characters/Bosses/BP_Giganto.CameraLockOnPoint` (`local.Target`))))))
  (`Controller.SetControlRotation` (`self.GetController`) (`KismetMathLibrary.RInterpTo` (`self.GetControlRotation`) (`KismetMathLibrary.MakeRotator` _returnvalue_roll _returnvalue_pitch _returnvalue_yaw) (`local.DeltaTime`) 5.0))
  (`self.SetCameraLocation` (`local.Target`) (`local.DeltaTime`)))

(fn `UserConstructionScript`)