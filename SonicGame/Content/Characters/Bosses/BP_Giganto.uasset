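; BP_Giganto is a boss character with body and head lock-on points for homing targeting.
; BeginPlay spawns a hidden homing icon attached to the head, with a function to toggle its visibility.
; SetHomingIconLocation reattaches it to the point nearest another actor by squared distance, but only head wins register because the first entry (body) never sets the component.
; GetHeadStompLocation returns a point offset above the head along the actor's up vector.
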(event `self.ReceiveBeginPlay`
  (bind _headlockonpoint (`self.HeadLockOnPoint`))
  (`KismetArrayLibrary.Array_Add` (`self.LockOnPoints`) (`self.BodyLockOnPoint`))
  (`KismetArrayLibrary.Array_Add` (`self.LockOnPoints`) _headlockonpoint)
  (bind _returnvalue (`|SpawnActorFromClass` "/Game/UI/HomingIconActor.HomingIconActor_C" (`KismetMathLibrary.MakeTransform` (`SceneComponent.K2_GetComponentLocation` _headlockonpoint)) "Undefined" "OverrideRootScale" null null))
  (bind _output_get (set `self.LockOnIcon` _returnvalue))
  (`self.K2_AttachToComponent` _output_get (`self.HeadLockOnPoint`) "None" "SnapToTarget" "SnapToTarget" "SnapToTarget" true)
  (`self.SetActorHiddenInGame` (`self.LockOnIcon`) true))

(fn `Get Closest Lock on Point`
  (params (OtherActor :type "Actor Object Reference"))
  (returns (Location :type "Vector Structure") (Component :type "SceneComponent Object Reference"))
  (locals (ClosestLocation :type "Vector Structure") (ClosestDistSq :type "Float (double-precision)") (ClosestComponent :type "SceneComponent Object Reference"))
  (bind _returnvalue (`SceneComponent.K2_GetComponentLocation` (`|GetArrayItem` (`self.LockOnPoints`))))
  (set `local.ClosestLocation` _returnvalue)
  (set `local.ClosestDistSq` (`KismetMathLibrary.Vector_DistanceSquared` _returnvalue (`self.K2_GetActorLocation` (`local.OtherActor`))))
  (for _array_element (`self.LockOnPoints`)
    (bind _returnvalue_2 (`SceneComponent.K2_GetComponentLocation` _array_element))
    (bind _returnvalue_3 (`KismetMathLibrary.Vector_DistanceSquared` _returnvalue_2 (`self.K2_GetActorLocation` (`local.OtherActor`))))
    (if (< _returnvalue_3 (`local.ClosestDistSq`))
      (set `local.ClosestComponent` _array_element)
      (set `local.ClosestDistSq` _returnvalue_3)
      (set `local.ClosestLocation` _returnvalue_2)))
  (return (`local.ClosestLocation`) (`local.ClosestComponent`)))

(fn `GetHeadStompLocation`
  (returns (Location :type "Vector Structure"))
  (return (+ (`SceneComponent.K2_GetComponentLocation` (`self.HeadLockOnPoint`)) (* (`self.GetActorUpVector`) 350.0))))

(fn `SetHomingIconLocation`
  (params (OtherActor :type "Actor Object Reference"))
  (locals (LockOnComponent :type "SceneComponent Object Reference"))
  (bind (_location _component) (`self.Get Closest Lock on Point` OtherActor))
  (`/Engine/EditorBlueprintResources/StandardMacros.IsValid` _component
    (:`Is Valid`
      (set `local.LockOnComponent` _component)
      (`self.K2_DetachFromActor` (`self.LockOnIcon`) "KeepWorld" "KeepWorld" "KeepRelative")
      (`self.K2_AttachToComponent` (`self.LockOnIcon`) (`local.LockOnComponent`) "None" "SnapToTarget" "SnapToTarget" "SnapToTarget" true))))

(fn `SetHomingIconVisibility`
  (params (Hidden :type Boolean))
  (`self.SetActorHiddenInGame` (`self.LockOnIcon`) Hidden))

(fn `UserConstructionScript`)