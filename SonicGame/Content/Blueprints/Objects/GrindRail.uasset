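; Grind rail actor that Sonic can grind along, built from a spline that can be a closed loop.
; The construction script lays a spline mesh segment between each pair of points, using their tangents and up vectors.
; EnterRail plays a landing sound and starts an attached grind sound on Sonic.
; ExitRail clears Sonic's rail state, stops that sound and briefly disables the rail's collision before re-enabling it.
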(event `self.ReceiveTick`
  (params (DeltaSeconds :type "Float (single-precision)")))

(event `EnterRail`
  (params (Player :type "Pawn Object Reference"))
  (bind _assonic (cast `/Game/Characters/Sonic` Player))
  (`GameplayStatics.PlaySoundAtLocation` "/Game/GeneralAudio/RailLand.RailLand" (`self.K2_GetActorLocation` _assonic) (struct) 0.75 1.0 0.0 null null null null)
  (bind _returnvalue (`GameplayStatics.SpawnSoundAttached` "/Game/GeneralAudio/RailGrind.RailGrind" (`SonicGameCharacter.SoundEffectComponent` _assonic) "None" (0.0 0.0 0.0) (struct) "KeepRelativeOffset" false 0.75 1.0 0.0 null null))
  (set `self.SoundReference` _returnvalue))

(event `ExitRail`
  (bind _soundreference (`self.SoundReference`))
  (bind _assonic (cast `/Game/Characters/Sonic` (`GameplayStatics.GetPlayerPawn` 0)))
  (set `SonicGameCharacter.CurrentRail` null _assonic)
  (set `SonicGameCharacter.bIsGrinding` false _assonic)
  (`self.SetActorEnableCollision` false)
  (`AudioComponent.Stop` _soundreference)
  (`ActorComponent.K2_DestroyComponent` _soundreference)
  (`KismetSystemLibrary.Delay` 0.5)
  (`self.SetActorEnableCollision` true))

(fn `GetSpineDataAtPoint`
  (params (Spline :type "SplineComponent Object Reference") (PointIndex :type Integer) (CoordinateSpace :type "ESplineCoordinateSpace Enum" :default "Local"))
  (returns (StartPosition :type "Vector Structure") (StartTangent :type "Vector Structure") (EndPosition :type "Vector Structure") (EndTangent :type "Vector Structure") (UpVector :type "Vector Structure"))
  (bind _returnvalue (+ PointIndex 1))
  (return (`SplineComponent.GetLocationAtSplinePoint` Spline PointIndex CoordinateSpace) (`SplineComponent.GetTangentAtSplinePoint` Spline PointIndex CoordinateSpace) (`SplineComponent.GetLocationAtSplinePoint` Spline _returnvalue CoordinateSpace) (`SplineComponent.GetTangentAtSplinePoint` Spline _returnvalue CoordinateSpace) (`SplineComponent.GetUpVectorAtSplinePoint` Spline PointIndex CoordinateSpace)))

(fn `UserConstructionScript`
  (bind _spline (`self.Spline`))
  (bind _closedloop (`self.ClosedLoop`))
  (`SplineComponent.SetClosedLoop` _spline _closedloop true)
  (for _index (range (+ (- (`SplineComponent.GetNumberOfSplinePoints` _spline) (`KismetMathLibrary.SelectInt` 1 2 _closedloop)) 1))
    (bind _returnvalue (`AddComponent|NODE_AddSplineMeshComponent-0`))
    (`StaticMeshComponent.SetStaticMesh` _returnvalue (`self.RailMesh`))
    (bind (_startposition _starttangent _endposition _endtangent _upvector) (`self.GetSpineDataAtPoint` (`self.Spline`) _index))
    (`SplineMeshComponent.SetStartAndEnd` _returnvalue _startposition _starttangent _endposition _endtangent true)
    (`SplineMeshComponent.SetSplineUpDir` _returnvalue _upvector true)))