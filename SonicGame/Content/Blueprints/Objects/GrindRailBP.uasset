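; Grind rail actor that Sonic grinds along, built from a designer-editable spline.
; The construction script lays a spline mesh per segment, optionally closing the loop, using start/end tangents and up vectors.
; EnterRail starts sparks and an attached grind sound.
; ExitRail clears Sonic's grind state, stops effects and briefly disables collision to avoid re-grabbing; RailJump stops the sound, plays a jump sound and exits.
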(event `self.ReceiveTick`
  (params (DeltaSeconds :type "Float (single-precision)")))

(event `self.EnterRail`
  (params (Player :type "SonicGameCharacter Object Reference"))
  (bind _assonic (cast `/Game/Characters/Sonic` Player))
  (set `SonicGameCharacter.bGrindJump` false _assonic)
  (`ActorComponent.Activate` (`/Game/Characters/Sonic.Sparks` _assonic) true)
  (`GameplayStatics.PlaySoundAtLocation` "/Game/GeneralAudio/RailLand.RailLand" (`self.K2_GetActorLocation` _assonic) (struct) 0.75 1.0 0.0 null null null null)
  (bind _returnvalue (`GameplayStatics.SpawnSoundAttached` "/Game/GeneralAudio/RailGrind.RailGrind" (`SonicGameCharacter.SoundEffectComponent` _assonic) "None" (0.0 0.0 0.0) (struct) "KeepRelativeOffset" false 0.75 1.0 0.0 null null))
  (set `self.SoundReference` _returnvalue))

(event `self.ExitRail`
  (bind _soundreference (`self.SoundReference`))
  (bind _assonic (cast `/Game/Characters/Sonic` (`GameplayStatics.GetPlayerPawn` 0)))
  (set `SonicGameCharacter.CurrentRail` null _assonic)
  (set `SonicGameCharacter.bIsGrinding` false _assonic)
  (set `SonicMovementComponent.bIgnoreGrindingDecel` true (cast `SonicMovementComponent` (`Character.CharacterMovement` _assonic) :!pure true))
  (`ActorComponent.Deactivate` (`/Game/Characters/Sonic.Sparks` _assonic))
  (`self.SetActorEnableCollision` false)
  (`/Engine/EditorBlueprintResources/StandardMacros.IsValid` _soundreference
    (:`Is Valid`
      (`AudioComponent.Stop` _soundreference)
      (`ActorComponent.K2_DestroyComponent` _soundreference))
    (:`Is Not Valid`
      _))
  (`KismetSystemLibrary.Delay` 0.5)
  (`self.SetActorEnableCollision` true))

(event `self.RailJump`
  (bind _soundreference (`self.SoundReference`))
  (`/Engine/EditorBlueprintResources/StandardMacros.IsValid` _soundreference
    (:`Is Valid`
      (`AudioComponent.Stop` _soundreference)
      (`ActorComponent.K2_DestroyComponent` _soundreference)
      (`GameplayStatics.PlaySoundAtLocation` "/Game/Models/Sonic/Audio/Effects/Modern/ModernJumpSnd.ModernJumpSnd" (`self.K2_GetActorLocation` (`GameplayStatics.GetPlayerPawn` 0)) (struct) 1.0 1.0 0.0 null null null null)
      (`self.ExitRail`))))

(fn `GetSpineDataAtPoint`
  (params (Spline :type "SplineComponent Object Reference") (PointIndex :type Integer) (CoordinateSpace :type "ESplineCoordinateSpace Enum" :default "Local"))
  (returns (StartPosition :type "Vector Structure") (StartTangent :type "Vector Structure") (EndPosition :type "Vector Structure") (EndTangent :type "Vector Structure") (UpVector :type "Vector Structure"))
  (bind _returnvalue (+ PointIndex 1))
  (return (`SplineComponent.GetLocationAtSplinePoint` Spline PointIndex CoordinateSpace) (`SplineComponent.GetTangentAtSplinePoint` Spline PointIndex CoordinateSpace) (`SplineComponent.GetLocationAtSplinePoint` Spline _returnvalue CoordinateSpace) (`SplineComponent.GetTangentAtSplinePoint` Spline _returnvalue CoordinateSpace) (`SplineComponent.GetUpVectorAtSplinePoint` Spline PointIndex CoordinateSpace)))

(fn `UserConstructionScript`
  (bind _closedloop (`self.ClosedLoop`))
  (bind _railspline (`self.RailSpline`))
  (`SplineComponent.SetClosedLoop` _railspline _closedloop true)
  (for _index (range (+ (- (`SplineComponent.GetNumberOfSplinePoints` _railspline) (`KismetMathLibrary.SelectInt` 1 2 _closedloop)) 1))
    (bind _returnvalue (`AddComponent|NODE_AddSplineMeshComponent-0`))
    (`StaticMeshComponent.SetStaticMesh` _returnvalue (`self.RailMesh`))
    (bind (_startposition _starttangent _endposition _endtangent _upvector) (`self.GetSpineDataAtPoint` (`self.RailSpline`) _index))
    (`SplineMeshComponent.SetStartAndEnd` _returnvalue _startposition _starttangent _endposition _endtangent true)
    (`SplineMeshComponent.SetSplineUpDir` _returnvalue _upvector true)))