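; RailCameraVolume is a trigger volume that switches the player's camera while grinding on rails.
; When a grinding SonicGameCharacter enters its box, it blends the controller's view target to an assigned camera.
; If flagged as an exit volume, it blends the view back to the character instead, using the same blend time.
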(event `self.Box.OnComponentBeginOverlap`
  (params (OverlappedComponent :type "PrimitiveComponent Object Reference") (OtherActor :type "Actor Object Reference") (OtherComp :type "PrimitiveComponent Object Reference") (OtherBodyIndex :type Integer) (bFromSweep :type Boolean) (SweepResult :type "HitResult Structure (by ref)"))
  (bind _cameraref (`self.CameraRef`))
  (bind _assonic_game_character (cast `SonicGameCharacter` OtherActor))
  (if (`SonicGameCharacter.bIsGrinding` _assonic_game_character)
    (bind _asplayer_controller (cast `PlayerController` (`Pawn.GetController` _assonic_game_character)))
    (if (`self.isExiting`)
      (`PlayerController.SetViewTargetWithBlend` _asplayer_controller _assonic_game_character (`self.BlendTime`) "VTBlend_Linear" 0.0 false)
      (else
        (`/Engine/EditorBlueprintResources/StandardMacros.IsValid` _cameraref
          (:`Is Valid`
            (`PlayerController.SetViewTargetWithBlend` _asplayer_controller _cameraref (`self.BlendTime`) "VTBlend_Linear" 0.0 false)))))))

(fn `UserConstructionScript`)