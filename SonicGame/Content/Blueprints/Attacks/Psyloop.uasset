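; Psyloop attack Blueprint built around a spline, apparently an unfinished prototype with no gameplay logic wired up.
; BeginPlay only runs a console command to toggle spline debug display, and the DisplaySpline event is empty.
; GetSpineDataAtPoint returns positions and tangents for a point and its successor, plus an up vector.
; Unconnected nodes would use it to add a spline mesh segment at the last point, but never run.
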(event `self.ReceiveBeginPlay`
  (`KismetSystemLibrary.ExecuteConsoleCommand` "show Splines" null))

(event `DisplaySpline`)

(fn `GetSpineDataAtPoint`
  (params (Spline :type "SplineComponent Object Reference") (PointIndex :type Integer) (CoordinateSpace :type "ESplineCoordinateSpace Enum" :default "Local"))
  (returns (StartPosition :type "Vector Structure") (StartTangent :type "Vector Structure") (EndPosition :type "Vector Structure") (EndTangent :type "Vector Structure") (UpVector :type "Vector Structure"))
  (bind _returnvalue (+ PointIndex 1))
  (return (`SplineComponent.GetLocationAtSplinePoint` Spline PointIndex CoordinateSpace) (`SplineComponent.GetTangentAtSplinePoint` Spline PointIndex CoordinateSpace) (`SplineComponent.GetLocationAtSplinePoint` Spline _returnvalue CoordinateSpace) (`SplineComponent.GetTangentAtSplinePoint` Spline _returnvalue CoordinateSpace) (`SplineComponent.GetUpVectorAtSplinePoint` Spline PointIndex CoordinateSpace)))

(fn `UserConstructionScript`)