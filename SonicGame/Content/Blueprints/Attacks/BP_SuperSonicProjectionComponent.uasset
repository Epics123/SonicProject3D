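; Component for BP_SuperSonic that spawns the projections used in the special attack finisher.
; On the spawn event it casts its owner, takes the right vector as the starting direction and uses the normalized direction to the lock-on target's head point as the rotation axis.
; It then passes the finisher actor class, count, distance and a fixed angle to SpawnProjectionInCircle to place the projections.
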(event `self.SpawnSpecialAttackFinisherProjections`
  (bind _asbp_super_sonic (cast `/Game/Characters/SuperSonic/BP_SuperSonic` (`self.GetOwner`)))
  (set `self.StartingDirection` (`Actor.GetActorRightVector` _asbp_super_sonic))
  (set `self.RotationAxis` (`KismetMathLibrary.Normal` (- (`self.K2_GetComponentLocation` (`/Game/Characters/Bosses/BP_Giganto.HeadLockOnPoint` (`/Game/Characters/SuperSonic/BP_SuperSonic.LockOnTarget` _asbp_super_sonic))) (`Actor.K2_GetActorLocation` _asbp_super_sonic))))
  (`self.SpawnProjectionInCircle` "/Game/Blueprints/Attacks/BP_SuperSonic_SpecialFinish.BP_SuperSonic_SpecialFinish_C" (`self.NumFinisherProjections`) (`self.SpawnDistance`) 45.0))