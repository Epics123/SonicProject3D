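; BP_SuperSonic_SpecialFinish is an attack actor, named for Super Sonic's special finish, that handles only its own movement.
; On BeginPlay, the Move timeline eases it toward StartLocation.
; SetTargetDirectionfromDistance projects a target along TargetDirection by the given distance, then the MoveToTarget timeline eases it there.
; Both moves use VInterpTo from the current location without sweep, feeding timeline Alpha in as DeltaTime.
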(event `self.ReceiveBeginPlay`
  (`self.MoveToTargetLocation`))

(event `self.MoveToTargetLocation`
  (bind (_direction _alpha) (`Timeline|Move` :!via `PlayFromStart`)
    (:`Update`
      (`self.K2_SetActorLocation` (`KismetMathLibrary.VInterpTo` (`self.K2_GetActorLocation`) (`self.StartLocation`) _alpha 5.0)))))

(event `self.SetTargetDirectionFromDistance`
  (params (Distance :type "Float (single-precision)"))
  (set `self.TargetLocation` (+ (`self.K2_GetActorLocation`) (* (`self.TargetDirection`) Distance)))
  (bind (_direction _alpha) (`Timeline|MoveToTarget` :!via `PlayFromStart`)
    (:`Update`
      (`self.K2_SetActorLocation` (`KismetMathLibrary.VInterpTo` (`self.K2_GetActorLocation`) (`self.TargetLocation`) _alpha (`self.InterpSpeed`))))))

(event `self.ReceiveTick`
  (params (DeltaSeconds :type "Float (single-precision)")))

(fn `UserConstructionScript`)